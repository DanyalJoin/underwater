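; BP_Water is a water actor that pairs an ocean surface with an underwater post-process effect.
; The construction script assigns the water and underwater materials, pushes foam, wave and refraction settings to the Water component, and scales the actor.
; It also builds the PostProcess settings from the underwater material with configurable blend radius and weight.
; On actor overlap, it writes the Water component's doubled world location into MP_Water's "Height Water" parameter.
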(event `self.ReceiveActorBeginOverlap`
  (params (OtherActor :type "Actor Object Reference"))
  (`KismetMaterialLibrary.SetVectorParameterValue` "/Game/UnderWater/DataMaterials/Water.MP_Water" "Height Water" (`KismetMathLibrary.Conv_VectorToLinearColor` (* (`SceneComponent.K2_GetComponentLocation` (`self.Water`)) 2.0))))

(fn `UserConstructionScript`
  (bind _water (`self.Water`))
  (`PrimitiveComponent.SetMaterial` (`self.UnderWaterP`) 0 (`self.Underwater Material`))
  (`PrimitiveComponent.SetMaterial` (`self.Water`) 0 (`self.WaterMaterial`))
  (`MeshComponent.SetScalarParameterValueOnMaterials` _water "Foam Scale" (`self.Foam Scale`))
  (`MeshComponent.SetScalarParameterValueOnMaterials` _water "Foam Speed" (`self.Foam Speed`))
  (`MeshComponent.SetScalarParameterValueOnMaterials` _water "Foam Fade Distance" (`self.Foam Distance`))
  (`MeshComponent.SetScalarParameterValueOnMaterials` _water "Wave1 Scale" (`self.Wave1 Scale`))
  (`MeshComponent.SetScalarParameterValueOnMaterials` _water "Wave2 Scale" (`self.Wave2 Scale`))
  (`MeshComponent.SetScalarParameterValueOnMaterials` _water "Wave1 Speed" (`self.Wave1 Speed`))
  (`MeshComponent.SetScalarParameterValueOnMaterials` _water "Wave2 Speed" (`self.Wave2 Speed`))
  (`MeshComponent.SetScalarParameterValueOnMaterials` _water "Refraction Scale" (`self.Refraction Scale`))
  (`MeshComponent.SetScalarParameterValueOnMaterials` _water "Refraction Speed" (`self.Refraction Speed`))
  (`self.SetActorScale3D` (`self.OceanScale`))
  (bind _output_get (set `self.PostProcess` (`self.PostProcess`)))
  (set `PostProcessComponent.Settings` (make `PostProcessSettings` :`WeightedBlendables` (`self.UnderwaterMaterial`)) _output_get)
  (set `PostProcessComponent.BlendRadius` (`self.UnderwaterBlendRadius`) _output_get)
  (set `PostProcessComponent.BlendWeight` (`self.UnderwaterBlendWeight`) _output_get))